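; Base wolf enemy character that plays a melee attack and damages the player on contact.
; Tick scans overlapping components for BP_MainCharacter and, when both sides allow a hit, passes attack damage to its BCController's AddLife, then clears CanHit.
; Attack plays the melee montage directly on the mesh and flags IsAttacking, while UpdateWalkSpeed sets the movement speed.
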(event `self.ReceiveActorBeginOverlap`
  (params (OtherActor :type "Actor Object Reference")))

(event `self.ReceiveTick`
  (params (DeltaSeconds :type "Float (single-precision)"))
  ;[1 1 1] Attack damage
  (for _array_element (`self.GetOverlappingComponents`)
    (bind _asbp_main_character (cast `/Game/Player/BP_MainCharacter` (`ActorComponent.GetOwner` _array_element)))
    (bind _bccontroller (`/Game/Player/BP_MainCharacter.BCController` _asbp_main_character))
    (if (and (`BCController.GetCanBeHit` _bccontroller) (`self.GetCanHit`))
      (`BaseController.AddLife` _bccontroller (`self.GetAttackDamage`))
      (`self.SetCanHit` false)
      (break))))

(fn `Attack`
  ;[1 1 1] Play Anim
  (`SkeletalMeshComponent.PlayAnimation` (`self.Mesh`) "/Game/Enemies/Enemy_Wolf/Enemy_Wolf_Base_Animation/ExoGame_Wolf_Attack_Melee_Montage.ExoGame_Wolf_Attack_Melee_Montage" false)
  (set `self.IsAttacking` true))

(fn `UpdateWalkSpeed`
  (params (Speed :type "Float (double-precision)"))
  (set `CharacterMovementComponent.MaxWalkSpeed` Speed (`self.CharacterMovement`)))

(fn `UserConstructionScript`)