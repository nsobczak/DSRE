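; BP_AreaEnterTrigger is a placeable area trigger that reports its area name when the main character overlaps it.
; A child-actor trigger box, scaled in the construction script, runs UpdateAreaName on BeginPlay and on overlap begin.
; That function finds an overlapping BP_MainCharacter and calls SetCurrentArea on its BCController.
; If the controller is not yet valid, a flag makes Tick retry until it is.
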(event `self.ReceiveBeginPlay`
  (bind _childactor (`ChildActorComponent.ChildActor` (`self.TriggerBox`)))
  (add `self.OnActorBeginOverlap` _childactor (delegate `OnTriggerBeginOverlap`))
  (`self.UpdateAreaName` _childactor))

(event `OnTriggerBeginOverlap` :!signature `self.OnActorBeginOverlap`
  (params (OverlappedActor :type "Actor Object Reference") (OtherActor :type "Actor Object Reference"))
  (`self.UpdateAreaName` OverlappedActor))

(event `self.ReceiveTick`
  (params (DeltaSeconds :type "Float (single-precision)"))
  (if (`self.NeedToBeUpdated`)
    (`self.UpdateAreaName` (`ChildActorComponent.ChildActor` (`self.TriggerBox`)))))

(event `self.ReceiveActorBeginOverlap`
  (params (OtherActor :type "Actor Object Reference")))

(fn `UpdateAreaName`
  (params (OverlapedActor :type "Actor Object Reference"))
  (for _array_element (`self.GetOverlappingActors` OverlapedActor "/Game/Player/BP_MainCharacter.BP_MainCharacter_C")
    (bind _asbp_main_character (cast `/Game/Player/BP_MainCharacter` _array_element))
    (bind _bccontroller (`/Game/Player/BP_MainCharacter.BCController` _asbp_main_character))
    (`/Engine/EditorBlueprintResources/StandardMacros.IsValid` _bccontroller
      (:`Is Valid`
        (`BCController.SetCurrentArea` _bccontroller (`self.AreaName`))
        (set `self.NeedToBeUpdated` false)
        (break))
      (:`Is Not Valid`
        (set `self.NeedToBeUpdated` true)))))

(fn `UserConstructionScript`
  (`SceneComponent.SetRelativeScale3D` (`self.TriggerBox`) (`self.TriggerRelativeScale`)))